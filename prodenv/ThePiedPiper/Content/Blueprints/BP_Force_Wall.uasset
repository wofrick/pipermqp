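; BP_Force_Wall is a moving wall that pushes the player along its path.
; The construction script sets its direction to the negative Y axis of its rotation.
; After a delay, Tick moves it with a swept offset at a set velocity and destroys it once its lifetime passes.
; Box overlap events flag contact with the player, who then receives the same swept offset each frame.
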(event `self.ReceiveBeginPlay`)

(event `self.ReceiveTick`
  (params (DeltaSeconds :type "Float (single-precision)"))
  (set `self.deltaTime` (+ (`self.deltaTime`) DeltaSeconds))
  (if (> (`self.deltaTime`) (`self.delay`))
    (`self.K2_AddActorWorldOffset` (* (`KismetMathLibrary.Normal` (`self.dirVector`)) (* DeltaSeconds (`self.velocity`))) true)
    (if (`self.collisionVar`)
      (`self.K2_AddActorWorldOffset` (`self.PlayerActor`) (* (`self.dirVector`) (* DeltaSeconds (`self.velocity`))) true false))
    (if (> (`self.deltaTime`) (`self.lifetime_sec`))
      (`self.K2_DestroyActor`))))

(event `self.Box.OnComponentBeginOverlap`
  (params (OtherActor :type "Actor Object Reference") (OtherComp :type "PrimitiveComponent Object Reference") (OtherBodyIndex :type Integer) (bFromSweep :type Boolean) (SweepResult :type "HitResult Structure (by ref)"))
  (if (== OtherActor (`self.PlayerActor`))
    (set `self.collisionVar` true)))

(event `self.Box.OnComponentEndOverlap`
  (params (OtherActor :type "Actor Object Reference") (OtherComp :type "PrimitiveComponent Object Reference") (OtherBodyIndex :type Integer))
  (if (== (`self.PlayerActor`) OtherActor)
    (set `self.collisionVar` false)))

(fn `UserConstructionScript`
  (set `self.dirVector` (* (`.Y` (`KismetMathLibrary.GetAxes` (`self.K2_GetActorRotation`))) -1.0)))