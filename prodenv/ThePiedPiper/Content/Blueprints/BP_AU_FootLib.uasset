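; Footstep audio actor that plays randomized step sounds for player character 0 while it moves on the ground.
; Tick accumulates a timer and plays the Audio component when it is idle and the timer exceeds Delay scaled by speed over max speed, so the threshold grows with speed.
; Each trigger resets the timer and assigns a random Samples entry after calling Play; standing still primes the timer to a fraction of Delay.
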(event `self.ReceiveBeginPlay`
  (`AudioComponent.SetSound` (`self.Audio`) "/Game/Audio/SFX/step_tile_3.step_tile_3"))

(event `self.ReceiveActorBeginOverlap`
  (params (OtherActor :type "Actor Object Reference")))

(event `self.ReceiveTick`
  (params (DeltaSeconds :type "Float (single-precision)"))
  (bind _returnvalue (`GameplayStatics.GetPlayerCharacter` 0))
  (bind _samples (`self.samples`))
  (bind _returnvalue_2 (`KismetMathLibrary.VSize` (`self.GetVelocity` _returnvalue)))
  (bind _returnvalue_3 (> _returnvalue_2 0.0))
  (set `self.timer` (+ (`self.timer`) DeltaSeconds))
  (if (and (not (`AudioComponent.IsPlaying` (`self.Audio`))) (`NavMovementComponent.IsMovingOnGround` (`Character.CharacterMovement` _returnvalue)) (> (`self.timer`) (* (`self.delay`) (/ _returnvalue_2 (`MovementComponent.GetMaxSpeed` (`Character.CharacterMovement` _returnvalue))))) _returnvalue_3)
    (`AudioComponent.Play` (`self.Audio`) 0.0)
    (set `self.timer` 0.0)
    (`AudioComponent.SetSound` (`self.Audio`) (`KismetArrayLibrary.Array_Get` _samples (`KismetMathLibrary.RandomInteger` (`KismetArrayLibrary.Array_Length` _samples))))
    (elif (not _returnvalue_3)
      (set `self.timer` (/ (`self.delay`) 12.0)))))

(fn `UserConstructionScript`)