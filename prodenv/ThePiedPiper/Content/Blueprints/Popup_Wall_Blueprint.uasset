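; Pop-up wall actor that rises out of its start position and knocks the player away when the player enters its trigger volume.
; Tick polls the trigger overlap and latches a toggle, then sweeps the wall upward at constant speed to a fixed height above its start.
; On the first rising frame it launches the player once, along the wall's initial Y axis with an added upward boost.
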(event `self.ReceiveBeginPlay`
  (set `self.startZ` (.z (`self.K2_GetActorLocation`)))
  (set `self.startDir` (* (`.Y` (`KismetMathLibrary.GetAxes` (`self.K2_GetActorRotation`))) 1.0)))

(event `self.ReceiveActorBeginOverlap`
  (params (OtherActor :type "Actor Object Reference")))

(event `self.ReceiveTick`
  (params (DeltaSeconds :type "Float (single-precision)"))
  (bind _player (`self.Player`))
  (if (`PrimitiveComponent.IsOverlappingActor` (`self.TriggerVolume`) _player)
    (set `self.WallToggle` true))
  (if (`self.WallToggle`)
    (if (< (.z (`self.K2_GetActorLocation`)) (+ (`self.startZ`) 500.0))
      (`self.K2_AddActorWorldOffset` (`KismetMathLibrary.MakeVector` 0.0 0.0 (* DeltaSeconds 1600.0)) true)
      (if (not (`self.ImpulseToggle`))
        (`Character.LaunchCharacter` _player (+ (* (`KismetMathLibrary.Normal` (`self.startDir`)) (`self.Launch Power`)) (0.0 0.0 200.0)) false false)
        (set `self.ImpulseToggle` true)))))

(fn `UserConstructionScript`)