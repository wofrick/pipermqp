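; Bridge actor that rises vertically once triggered by the Piper actor, after a delay and up to a maximum height.
; Tick accumulates a timer while rising, then teleports the actor upward at a constant, frame-rate-independent speed.
; The trigger check runs on Tick's false branch, reading the Box overlap's OtherActor output, while the overlap event itself executes nothing.
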(event `self.ReceiveBeginPlay`)

(event `self.ReceiveTick`
  (params (DeltaSeconds :type "Float (single-precision)"))
  (if (`self.IsRising`)
    (set `self.timer` (+ DeltaSeconds (`self.timer`))))
  (if (and (`self.IsRising`) (< (.z (`self.K2_GetActorLocation`)) (`self.maxHeight`)) (> (`self.timer`) (`self.riseDelay`)))
    (`self.K2_AddActorWorldOffset` (`KismetMathLibrary.MakeVector` 0.0 0.0 (* 500.0 DeltaSeconds)) false true)
    (elif (== (`self.Piper`) (stale `self.Box.OnComponentBeginOverlap` OtherActor))
      (set `self.IsRising` true))))

(event `self.Box.OnComponentBeginOverlap`
  (params (OtherActor :type "Actor Object Reference") (OtherComp :type "PrimitiveComponent Object Reference") (OtherBodyIndex :type Integer) (bFromSweep :type Boolean) (SweepResult :type "HitResult Structure (by ref)")))

(fn `UserConstructionScript`)