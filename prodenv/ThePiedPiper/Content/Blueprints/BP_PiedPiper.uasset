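; BP_PiedPiper is an AI-moved actor that travels along an ordered array of waypoint targets.
; Each tick it issues a simple move toward the current target.
; Within 200 units, if that target's Go flag is set, it waits the target's Delay before advancing the index, stopping at the last one.
; It teleports to any new target flagged Teleport; the TimeElapsed accumulator is disconnected.
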(event `self.ReceiveTick`
  (params (DeltaSeconds :type "Float (single-precision)"))
  (bind _targets (`self.targets`))
  (bind _item (`KismetArrayLibrary.Array_Get` _targets (`self.pathIndex`)))
  (bind _item_2 (`KismetArrayLibrary.Array_Get` (`self.targets`) (`self.pathIndex`)))
  (`NavigationSystem.SimpleMoveToLocation` (`self.GetController`) (`self.K2_GetActorLocation` _item))
  (if (and (< (`self.GetDistanceTo` _item) 200.0) (< (`self.pathIndex`) (- (`KismetArrayLibrary.Array_Length` _targets) 1)) (`/Game/Blueprints/BP_Path_Node.go` _item))
    (`KismetSystemLibrary.Delay` (`KismetMathLibrary.Conv_IntToDouble` (`/Game/Blueprints/BP_Path_Node.delay` _item)))
    (set `self.timeElapsed` 0.0)
    (set `self.pathIndex` (+ (`self.pathIndex`) 1))
    (if (`/Game/Blueprints/BP_Path_Node.teleport` _item_2)
      (`self.K2_SetActorLocation` (`self.K2_GetActorLocation` _item_2) false true))))

(fn `UserConstructionScript`)