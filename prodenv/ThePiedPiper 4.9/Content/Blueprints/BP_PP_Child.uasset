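; BP_PP_Child is a controlled actor, likely a pawn, that walks through an ordered list of target actors.
; Each tick, its controller issues a simple move toward the current target's location.
; When the actor comes within a short distance of that target, the path index advances until it reaches the last one, where it stops advancing.
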(event `self.ReceiveTick`
  (params (DeltaSeconds :type "Float (single-precision)"))
  (bind _targets (`self.targets`))
  (bind _item (`KismetArrayLibrary.Array_Get` _targets (`self.pathIndex`)))
  (`NavigationSystem.SimpleMoveToLocation` (`self.GetController`) (`self.K2_GetActorLocation` _item))
  (if (and (< (`self.GetDistanceTo` _item) 100.0) (< (`self.pathIndex`) (- (`KismetArrayLibrary.Array_Length` _targets) 1)))
    (set `self.pathIndex` (+ (`self.pathIndex`) 1))))

(fn `UserConstructionScript`)