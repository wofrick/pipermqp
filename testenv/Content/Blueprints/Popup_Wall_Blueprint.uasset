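; Popup wall actor that rises out of the ground when the player comes within range and knocks them away.
; Each tick it checks distance to the player and latches a toggle once close enough.
; While latched, it sweeps itself upward until its mesh reaches a height limit.
; On the first rise step it launches the player once along a fixed world-space sideways and upward velocity.
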(event `self.ReceiveBeginPlay`)

(event `self.ReceiveActorBeginOverlap`
  (params (OtherActor :type "Actor Object Reference")))

(event `self.ReceiveTick`
  (params (DeltaSeconds :type "Float (single-precision)"))
  (bind _player (`self.Player`))
  (if (< (`self.GetDistanceTo` _player) 500.0)
    (set `self.WallToggle` true))
  (if (`self.WallToggle`)
    (if (< (.z (`SceneComponent.K2_GetComponentLocation` (`self.StaticMeshComponent`))) 100.0)
      (`self.K2_AddActorWorldOffset` (`KismetMathLibrary.MakeVector` 0.0 0.0 (* DeltaSeconds 1600.0)) true)
      (if (not (`self.ImpulseToggle`))
        (`Character.LaunchCharacter` _player (0.0 1600.0 700.0) false false)
        (set `self.ImpulseToggle` true)))))

(fn `UserConstructionScript`)